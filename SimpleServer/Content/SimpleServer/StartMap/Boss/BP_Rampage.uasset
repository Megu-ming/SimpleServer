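; BP_Rampage is a boss character with a normal attack and a rock launch event.
; It disables its left and right hand colliders on BeginPlay.
; NormalAttack plays a slowed combo montage, while LaunchRock calls PlayMontage with no montage assigned.
; Both reset CurrentState to the enum's first entry when the montage completes.
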(event Custom|NormalAttack
  (Animation|Montage|PlayMontage (Variables|Character|GetMesh) "/Game/SimpleServer/StartMap/Boss/Animation/Attack_Combo_Montage.Attack_Combo_Montage" 0.8
    (:OnCompleted
      (Variables|Default|SetCurrentState "NewEnumerator0"))))

(event Custom|LaunchRock
  (Animation|Montage|PlayMontage (Variables|Character|GetMesh) 0
    (:OnCompleted
      (Variables|Default|SetCurrentState "NewEnumerator0"))))

(event EventBeginPlay
  (Collision|SetCollisionEnabled (Variables|Default|GetRightHandCollider) "NoCollision")
  (Collision|SetCollisionEnabled (Variables|Default|GetLeftHandCollider) "NoCollision"))

(fn ConstructionScript)