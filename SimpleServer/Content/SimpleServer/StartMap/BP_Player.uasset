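; Player character Blueprint that handles stamina-based running and creates the combat HUD, passing it the StatusComponent.
; Holding evade/run while moving switches to run speed after a stamina check, draining stamina per trigger until release or exhaustion restores jog speed.
; A timeline serves as the regeneration tick, paused while running and restarted through a gated delay helper once no montage plays.
; Both drain and regeneration refresh the HUD stamina bar.
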(event Custom|RefreshStaminaRegeneration
  (params (StartStaminaRegeneration :type Boolean))
  (if StartStaminaRegeneration
    (Timeline|StaminaRegenerationLooper PlayFromStart
      (:Update
        (Utilities|StaminaRegenTick)))
    (else
      (Timeline|StaminaRegenerationLooper Stop))))

(event Custom|StopRunning
  (Variables|/Script/Engine.CharacterMovementComponent|SetMaxWalkSpeed (Variables|Character|GetCharacterMovement) (Variables|/Game/SimpleServer/StartMap/StatusComponent.StatusComponent_C|GetJogSpeed (Variables|Default|GetStatusComponent)))
  (if (not (Class|AnimInstance|IsAnyMontagePlaying (Components|SkeletalMesh|GetAnimInstance (Variables|Character|GetMesh))))
    (Variables|Default|SetCurrentPlayerState "NewEnumerator0")
    (Utilities|HandleStaminaRegen true 0.0)))

(event Input|EnhancedActionEvents|EnhancedInputActionIA_Evade_Run
  (params (ActionValue :type Boolean) (ElapsedSeconds :type Float%20%28double-precision%29) (TriggeredSeconds :type Float%20%28double-precision%29) (InputAction :type Input%20Action%20Object%20Reference :default "/Game/SimpleServer/StartMap/Input/IA_Evade_Run.IA_Evade_Run"))
  (:Triggered
    (if (and (PrivatePure|HasMovementKeyInput) (Variables|Default|GetMovementInput))
      (if (Utilities|Enum|Equal(Enum) (Variables|Default|GetCurrentPlayerState) "NewEnumerator1")
        (Utilities|RunTick :!label _label)
        (elif (PrivatePure|CheckforStamina 2e+01)
          (Utilities|HandleStaminaRegen false 0.75)
          (Variables|/Script/Engine.CharacterMovementComponent|SetMaxWalkSpeed (Variables|Character|GetCharacterMovement) (Variables|/Game/SimpleServer/StartMap/StatusComponent.StatusComponent_C|GetRunSpeed (Variables|Default|GetStatusComponent)))
          (Variables|Default|SetCurrentPlayerState "NewEnumerator1")
          (goto _label)
          (else
            (Variables|/Script/Engine.CharacterMovementComponent|SetMaxWalkSpeed (Variables|Character|GetCharacterMovement) (Variables|/Game/SimpleServer/StartMap/StatusComponent.StatusComponent_C|GetJogSpeed (Variables|Default|GetStatusComponent)) :!label _label_2)
            (if (not (Class|AnimInstance|IsAnyMontagePlaying (Components|SkeletalMesh|GetAnimInstance (Variables|Character|GetMesh))))
              (Variables|Default|SetCurrentPlayerState "NewEnumerator0")
              (Utilities|HandleStaminaRegen true 0.0)))))))
  (:Completed
    (goto _label_2)))

(event EventBeginPlay
  (Utilities|FlowControl|Sequence
    (:then_0
      (bind _returnvalue (UserInterface|CreateWidget "/Game/SimpleServer/StartMap/Widget/UI_PlayerCombat.UI_PlayerCombat_C" 0 (Variables|Default|GetStatusComponent)))
      (bind _output_get (Variables|Default|SetUIPlayerCombat _returnvalue))
      (UserInterface|Viewport|AddtoViewport _output_get 0))
    (:then_1
      (CallFunction|RefreshStaminaRegeneration true))))

(fn ConstructionScript)

(fn HasMovementKeyInput
  (return (Utilities|Operators|NotEqual(!=) :A (Pawn|Components|PawnMovement|GetLastInputVector (Variables|Character|GetCharacterMovement)) :ErrorTolerance 0.001)))

(fn CheckforStamina
  (params (StaminaNeeded :type Float%20%28double-precision%29))
  (return (>= (Variables|/Game/SimpleServer/StartMap/StatusComponent.StatusComponent_C|GetCurrentStamina (Variables|Default|GetStatusComponent)) StaminaNeeded)))