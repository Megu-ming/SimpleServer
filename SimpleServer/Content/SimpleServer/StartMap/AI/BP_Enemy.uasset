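; BP_Enemy is an AI enemy pawn that wanders briefly and then chases the player on sight.
; On BeginPlay it sets its walk speed and moves once to a random navigable point near its spawn location.
; When PawnSensing sees a PlayerCharacter, it stores that player and calls FollowPlayer, which uses AIMoveTo to pursue the player actor.
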(event OnSeePawn(PawnSensing)
  (params (Pawn :type Pawn%20Object%20Reference))
  (bind _asplayer_character (Utilities|Casting|CastToPlayerCharacter Pawn))
  (Variables|Default|SetPlayerCharacter _asplayer_character)
  (CallFunction|FollowPlayer))

(event Custom|FollowPlayer
  (AI|AIMoveTo self "0, 0, 0" (Variables|Default|GetPlayerCharacter) 5.0 false))

(event EventBeginPlay
  (Variables|/Script/Engine.CharacterMovementComponent|SetMaxWalkSpeed (Variables|Character|GetCharacterMovement) 2.5e+02)
  (bind _randomlocation (Class|NavigationSystemV1|GetRandomLocationinNavigableRadius (Transformation|GetActorLocation) 5e+02 0 0))
  (AI|AIMoveTo self _randomlocation 0 5.0 false))

(event Collision|EventActorBeginOverlap
  (params (OtherActor :type Actor%20Object%20Reference)))

(event EventTick
  (params (DeltaSeconds :type Float%20%28single-precision%29)))

(fn ConstructionScript)